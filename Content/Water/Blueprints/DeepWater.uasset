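; Deep water volume actor that switches the player character into and out of swimming.
; A surface plane overlap starts swimming and disables its collision until the player's actor end overlap stops swimming and re-enables it.
; When the camera leaves the box and the player is out, a timeline fades a droplet effect.
; The construction script feeds exposed depth, wave, colour and texture settings into a dynamic water material.
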(event OnComponentEndOverlap(Box)
  (params (OverlappedComponent :type Primitive%20Component%20Object%20Reference) (OtherActor :type Actor%20Object%20Reference) (OtherComp :type Primitive%20Component%20Object%20Reference) (OtherBodyIndex :type Integer))
  ;[1 1 1] Droplet Effect
  (if (Components|ComponentHasTag OtherComp "Camera")
    (Utilities|FlowControl|Delay 0.2)
    (if (not (Variables|Default|GetPlayerIn))
      (Variables|/Script/Engine.PostProcessComponent|SetbEnabled (Variables|Default|GetDropsEffect) true)
      (bind _newtrack_0 (Timeline|FadoutTimeline PlayFromStart)
        (:Update
          (Variables|/Script/Engine.PostProcessComponent|SetBlendWeight (Variables|Default|GetDropsEffect) (Math|Float|Lerp 1.0 0.0 _newtrack_0)))
        (:Finished
          (Variables|/Script/Engine.PostProcessComponent|SetbEnabled (Variables|Default|GetDropsEffect) true))))))

(event OnComponentBeginOverlap(Plane)
  (params (OverlappedComponent :type Primitive%20Component%20Object%20Reference) (OtherActor :type Actor%20Object%20Reference) (OtherComp :type Primitive%20Component%20Object%20Reference) (OtherBodyIndex :type Integer) (bFromSweep :type Boolean) (SweepResult :type Hit%20Result%20Structure%20%28by%20ref%29))
  ;[1 1 1] Start swimming
  (if (Actor|ActorHasTag OtherActor "Player")
    (if (not (Components|ComponentHasTag OtherComp "Camera"))
      (bind _asbp_third_person_character (Utilities|Casting|CastToBP_ThirdPersonCharacter OtherActor))
      (Default|StartSwimming _asbp_third_person_character)
      (Variables|Default|SetPlayerIn true)
      (Collision|SetCollisionEnabled (Variables|Default|GetPlane) "NoCollision") ; Turn off plane collision while swimming so it won't trigger again
    )))

(event Collision|EventActorEndOverlap
  (params (OtherActor :type Actor%20Object%20Reference))
  ;[1 1 1] Stop swimming
  (if (Actor|ActorHasTag OtherActor "Player")
    (if (Variables|Default|GetPlayerIn)
      (bind _asbp_third_person_character (Utilities|Casting|CastToBP_ThirdPersonCharacter OtherActor))
      (Default|StopSwimming _asbp_third_person_character)
      (Variables|Default|SetPlayerIn false)
      (Collision|SetCollisionEnabled (Variables|Default|GetPlane) "QueryOnly") ; Reenable plane collision so swimming state can be triggered again
    )))

(fn ConstructionScript
  (bind _watersurface (Variables|Default|GetWaterSurface))
  (bind _returnvalue (Rendering|Material|CreateDynamicMaterialInstance (Variables|Default|GetWaterSurface) 0 "/Game/Water/Assets/Materials/WaterWaveMat_Inst.WaterWaveMat_Inst" "None" :!class /Script/Engine.PrimitiveComponent))
  (Variables|Waves|SetWaveInst _returnvalue)
  (Rendering|Material|SetMaterial (Variables|Default|GetWaterSurface) 0 (Variables|Waves|GetWaveInst))
  ;[1 1 1] Scalar Parameters
  (Rendering|Material|SetScalarParameterValueonMaterials _watersurface "CompleteOpacityDepth(cm)" (Variables|Waves|GetCompleteOpacityDepth))
  (Rendering|Material|SetScalarParameterValueonMaterials _watersurface "WaveHeight" (Variables|Waves|GetWaveHeight))
  (Rendering|Material|SetScalarParameterValueonMaterials _watersurface "WaveSpeed" (Variables|Waves|GetWaveSpeed))
  ;[1 1 1] Vector Parameters
  (Rendering|Material|SetVectorParameterValueonMaterials _watersurface "ShallowsColour" (Variables|Waves|GetShallowColour))
  (Rendering|Material|SetVectorParameterValueonMaterials _watersurface "DepthsColour" (Variables|Waves|GetDeepColour))
  ;[1 1 1] Texture Parameters
  (Rendering|Material|SetTextureParameterValue (Variables|Waves|GetWaveInst) "WaveTextureSample" (Variables|Waves|GetWaveSample)))