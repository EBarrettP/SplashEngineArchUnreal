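; FloatingObject is a buoyancy Blueprint that pushes a mesh upward at float points that sit in water.
; The construction script creates a configurable number of tiny box components on the mesh, placed at editable relative positions.
; CheckFloatState collects points at or below a given water height and sets Underwater when their count reaches half the total.
; UpwardForce applies a vertical impulse at each submerged point, summing wave height and floating power.
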(event Custom|CheckFloatState
  (params (WaterHeight :type Float%20%28double-precision%29))
  (bind _floatpoints (Variables|FloatPoints|GetFloatPoints))
  (Utilities|Array|Clear (Variables|Default|GetFloatPointUnderwater))
  (Variables|Default|SetFloatCounter 0)
  (for _array_element _floatpoints
    (if (<= (.z (Transformation|GetWorldLocation _array_element)) WaterHeight)
      (Variables|Default|SetFloatCounter (+ (Variables|Default|GetFloatCounter) 1))
      (Utilities|Array|Add (Variables|Default|GetFloatPointUnderwater) _array_element)))
  (if (>= (Variables|Default|GetFloatCounter) (/ (Utilities|Array|Length _floatpoints) 2))
    (Variables|Default|SetUnderwater true)
    (else
      (Variables|Default|SetUnderwater false))))

(event Custom|UpwardForce
  (params (WaveHeight :type Float%20%28double-precision%29) (FloatingPower :type Float%20%28double-precision%29))
  (for _array_element (Variables|Default|GetFloatPointUnderwater)
    (Physics|AddImpulseatLocation (Variables|Default|GetMesh) (Math|Vector|MakeVector 0.0 0.0 (+ WaveHeight FloatingPower)) (Transformation|GetWorldLocation _array_element) "None")))

(fn ConstructionScript
  (bind _floatpoints (Variables|FloatPoints|GetFloatPoints))
  (Utilities|Array|Clear (Variables|FloatPoints|GetFloatPoints))
  (if (!= 0 (Variables|FloatPoints|GetNumberOfFloatPoints))
    (for _index (range 1 (Variables|FloatPoints|GetNumberOfFloatPoints))
      (bind _returnvalue (AddComponent|AddBoxComponent true))
      (Utilities|Array|Add (Variables|FloatPoints|GetFloatPoints) _returnvalue)
      (Transformation|AttachComponentToComponent _returnvalue (Variables|Default|GetMesh) "None" "KeepRelative" "KeepRelative" "KeepRelative" false)
      (Transformation|SetRelativeScale3D _returnvalue "0.010000,0.010000,0.010000")
      (Variables|/Script/Engine.PrimitiveComponent|SetCanCharacterStepUpOn _returnvalue "ECB_No"))
    (Utilities|Array|Resize (Variables|FloatPoints|GetFloatPointRelativePosition) (Utilities|Array|Length _floatpoints))
    (for (_array_element _array_index) _floatpoints
      (Transformation|SetRelativeLocation _array_element (Utilities|Array|Get(acopy) (Variables|FloatPoints|GetFloatPointRelativePosition) _array_index) false false))))